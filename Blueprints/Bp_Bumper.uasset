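; Pinball bumper actor that knocks a Bp_ball away when overlapped and awards score through PinballGameMode.
; Bump applies a velocity-change impulse along the bumper-to-ball direction and plays an attached collision sound.
; The BumperLerp timeline animates the bumper mechanism vertically while driving the point light and the glow parameter on a dynamic material created in the construction script.
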(event `self.ReceiveActorBeginOverlap`
  (params (OtherActor :type "Actor Object Reference"))
  (bind _asbp_ball (cast `/Game/Blueprints/Bp_ball` OtherActor))
  (`self.Bump` _asbp_ball))

(event `Bump`
  (params (ball :type "/Game/Blueprints/Bp_ball Object Reference"))
  (`PrimitiveComponent.AddImpulse` (`/Game/Blueprints/Bp_ball.ball` ball) (* (`KismetMathLibrary.GetDirectionUnitVector` (`self.K2_GetActorLocation`) (`self.K2_GetActorLocation` ball)) 3500.0) "None" true)
  (`GameplayStatics.SpawnSoundAttached` "/Game/Assets/Sounds/Bumpercollision.Bumpercollision" (`self.Bumper_mesh`) "None" (0.0 0.0 0.0) (struct) "KeepRelativeOffset" false 1.0 1.0 0.0 null null)
  (bind _aspinball_game_mode (cast `/Game/Blueprints/PinballGameMode` (`GameplayStatics.GetGameMode`))
    (:`then`
      (`/Game/Blueprints/PinballGameMode.AddScore` _aspinball_game_mode 20.0)
      (bind (_direction _bump_alpha) (`Timeline|BumperLerp` :!via `PlayFromStart` :!label _label)
        (:`Update`
          (`SceneComponent.K2_SetRelativeLocation` (`self.Bumper_mech`) (`KismetMathLibrary.VLerp` (0.0 0.0 0.0) (0.0 0.0 -60.0) _bump_alpha) false false)
          (`LightComponent.SetIntensity` (`self.PointLight`) (`KismetMathLibrary.Lerp` 0.0 5000.0 _bump_alpha))
          (`MaterialInstanceDynamic.SetScalarParameterValue` (`self.BumperTopMID`) "Lightup" (`KismetMathLibrary.Lerp` 0.0 50.0 _bump_alpha)))))
    (:`CastFailed`
      (goto _label :!via `PlayFromStart`))))

(fn `UserConstructionScript`
  (bind _returnvalue (`PrimitiveComponent.CreateDynamicMaterialInstance` (`self.Bumper_mesh`) 1 "/Game/Assets/M_bumper_material.M_bumper_material" "None"))
  (set `self.BumperTopMID` _returnvalue))